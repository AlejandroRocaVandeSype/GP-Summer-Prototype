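; BP_OffsetNote sets up a fixed-melody voice pitch minigame built from an array of semitone note offsets.
; On BeginPlay it creates UMG_OffsetNote, sizes its rows to the offset range and adds each note.
; VoicePitchData pitch events update the current-note indicator and tint the first note while CurrentNote is zero.
; Hold-to-advance progression and the timer reset are unwired; the pitch-match condition is a constant true.
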(event `self.ReceiveBeginPlay`
  (bind _noteoffset (`self.NoteOffset`))
  ;[0 1 0.09038] Initialising fixed melody minigame
  (`|ExecutionSequence`
    (:`then_0`
      ;;[1 1 1] Initialising widget
      ;;;[1 1 1] Creating melody widget
      (bind _returnvalue (`|CreateWidget` "/Game/ArtAssets/UI/UMG_OffsetNote.UMG_OffsetNote_C"))
      (bind _output_get (set `self.Widget` _returnvalue))
      (`UserWidget.AddToViewport` _output_get 0)
      ;;;[1 1 1] Setting range of notes in array
      (set `/Game/ArtAssets/UI/UMG_OffsetNote.MaxRows` (`KismetMathLibrary.Abs_Int` (- (`.MinValue` (`KismetMathLibrary.MinOfIntArray` _noteoffset)) (`.MaxValue` (`KismetMathLibrary.MaxOfIntArray` _noteoffset)))) (`self.Widget`))
      ;;;[1 1 1] Initialising notes
      (for (_array_element _array_index) (`self.NoteOffset`)
        (`/Game/ArtAssets/UI/UMG_OffsetNote.AddNote` (`self.Widget`) _array_element (`.MinValue` (`KismetMathLibrary.MinOfIntArray` (`self.NoteOffset`))) _array_index)))
    (:`then_1`
      ;;[1 1 1] Binding voice pitch data events
      (add `/Game/Blueprints/AudioAnalysis/BP_VoicePitchAnalyzer.OnVoicePitchChange` (`self.VoicePitchData`) (delegate `VoicePitchChange`))
      (add `/Game/Blueprints/AudioAnalysis/BP_VoicePitchAnalyzer.OnVoiceInputEnd` (`self.VoicePitchData`) (delegate `ResetTimeNoteHeld`)))))

(event `ResetTimeNoteHeld`
  ;[1 0.5418 0.2977] Resetting time note held
)

(event `VoicePitchChange`
  (params (NoteNumber :type Integer) (NoteName :type "EMusicalNoteName Enum" :default "C") (NoteColor :type "LinearColor Structure"))
  ;[1 0.8357 0.1739] Updating melody widget on voice pitch change
  (`|ExecutionSequence`
    (:`then_0`
      ;;[1 1 1] Updating melody widget current note indicator
      (`/Game/ArtAssets/UI/UMG_CurrentNote.UpdateCurrentNote` (`/Game/ArtAssets/UI/UMG_OffsetNote.UMG_CurrentNote` (`self.Widget`)) NoteName))
    (:`then_1`
      (if (== (`self.CurrentNote`) 0)
        (`/Game/ArtAssets/UI/UMG_Note.SetColour` (`|GetArrayItem` (`/Game/ArtAssets/UI/UMG_OffsetNote.Notes` (`self.Widget`))) NoteColor)))))

(fn `UserConstructionScript`)