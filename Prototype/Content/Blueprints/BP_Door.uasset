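; BP_Door is a door the player can open only by singing nearby, with SetOpenDoor acting only while the player is in range.
; Tick polls the 2D distance to the BP_FPCharacter mesh and tells BP_FixedMelody to add or remove its melody widget as the player enters or leaves range.
; Once opened, the mesh slides along the MoveDirection forward vector each frame until a Delay in Tick clears the open flag.
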(event `self.ReceiveBeginPlay`
  (bind _returnvalue (`GameplayStatics.GetActorOfClass` "/Game/Blueprints/Character/BP_FPCharacter.BP_FPCharacter_C"))
  (set `self.PlayerCharacter` _returnvalue))

(event `self.ReceiveTick`
  (params (DeltaSeconds :type "Float (single-precision)"))
  (bind _issingingactive (`self.IsSingingActive`))
  (`|ExecutionSequence`
    (:`then_0`
      (if (`self.IsDoorOpen`)
        (`self.OpenDoor` DeltaSeconds)
        (`KismetSystemLibrary.Delay` 10.0)
        (set `self.IsDoorOpen` false)))
    (:`then_1`
      (if (< (`KismetMathLibrary.Vector_Distance2D` (`SceneComponent.K2_GetComponentLocation` (`self.DoorMesh`)) (`SceneComponent.K2_GetComponentLocation` (`Character.Mesh` (`self.PlayerCharacter`)))) (`self.ValidSingingDist`))
        (set `self.IsCloseToDoor` true)
        (if (not _issingingactive)
          (bind _returnvalue (`GameplayStatics.GetActorOfClass` "/Game/Blueprints/Audio/AudioAnalysis/BP_FixedMelody.BP_FixedMelody_C"))
          (`/Engine/EditorBlueprintResources/StandardMacros.IsValid` _returnvalue
            (:`Is Valid`
              (`/Game/Blueprints/Audio/AudioAnalysis/BP_FixedMelody.OnAddMelodyWidget` _returnvalue)
              (set `self.IsSingingActive` true))))
        (elif _issingingactive
          (set `self.IsCloseToDoor` false)
          (set `self.IsSingingActive` false)
          (bind _returnvalue_2 (`GameplayStatics.GetActorOfClass` "/Game/Blueprints/Audio/AudioAnalysis/BP_FixedMelody.BP_FixedMelody_C"))
          (`/Engine/EditorBlueprintResources/StandardMacros.IsValid` _returnvalue_2
            (:`Is Valid`
              (`/Game/Blueprints/Audio/AudioAnalysis/BP_FixedMelody.OnRemoveMelodyWidget` _returnvalue_2))))))))

(fn `OpenDoor`
  (params (DeltaSeconds :type "Float (double-precision)"))
  (`SceneComponent.K2_SetWorldLocation` (`self.DoorMesh`) (+ (* (* DeltaSeconds 100.0) (`SceneComponent.GetForwardVector` (`self.MoveDirection`))) (`SceneComponent.K2_GetComponentLocation` (`self.DoorMesh`))) false false))

(fn `SetOpenDoor`
  ;[1 1 1] Only if singing close to the door it can be opened
  (if (`self.IsCloseToDoor`)
    (set `self.IsDoorOpen` true)))

(fn `UserConstructionScript`)