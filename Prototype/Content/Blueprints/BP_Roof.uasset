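; BP_Roof is a roof actor whose static mesh slides along its own up vector when triggered.
; The OnMoveRoof event sets a MoveBall flag, and Tick then moves the mesh at a fixed, frame-rate-independent speed without sweeping.
; A Delay inside Tick clears the flag after ten seconds, ending the movement.
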(event `OnMoveRoof`
  (set `self.MoveBall` true))

(event `self.ReceiveTick`
  (params (DeltaSeconds :type "Float (single-precision)"))
  (if (`self.MoveBall`)
    (`SceneComponent.K2_SetWorldLocation` (`self.StaticMesh`) (+ (* (* DeltaSeconds 350.0) (`SceneComponent.GetUpVector` (`self.StaticMesh`))) (`SceneComponent.K2_GetComponentLocation` (`self.StaticMesh`))) false false)
    (`KismetSystemLibrary.Delay` 10.0)
    (set `self.MoveBall` false)))

(fn `UserConstructionScript`)