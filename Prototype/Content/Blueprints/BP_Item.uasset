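; BP_Item is a world item actor that can be picked up.
; Its construction script applies the configured mesh and material to the Mesh component and sizes the ItemCollision box from CollisionSize.
; The Pickup event prints a message and destroys the actor, with no inventory or other effect.
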(event `/Game/Blueprints/BPI_Items.Pickup`
  (`KismetSystemLibrary.PrintString` "Item Picked Up!")
  (`self.K2_DestroyActor`))

(fn `UserConstructionScript`
  (bind _mesh (`self.Mesh`))
  (`StaticMeshComponent.SetStaticMesh` _mesh (`self.ItemMesh`))
  (`PrimitiveComponent.SetMaterial` _mesh 0 (`self.Material`))
  (`BoxComponent.SetBoxExtent` (`self.ItemCollision`) (`self.CollisionSize`) true))