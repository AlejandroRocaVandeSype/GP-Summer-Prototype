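; BP_Light is a light fixture actor that pairs an emissive plane mesh with a rect light and switches on after a delay.
; BeginPlay puts a dynamic M_Emissive instance on the plane and, if On is set, applies its Intensity immediately.
; Tick accumulates time and, once past TurnOnAfter, sets the emissive intensity and a fixed rect light intensity every frame, regardless of On.
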(event `self.ReceiveBeginPlay`
  (bind _returnvalue (`KismetMaterialLibrary.CreateDynamicMaterialInstance` "/Game/ArtAssets/Materials/M_Emissive.M_Emissive" "LightMaterial"))
  (bind _output_get (set `self.LightMaterial` _returnvalue))
  (`PrimitiveComponent.SetMaterial` (`self.GP_LevelBlockoutPieces_SM_LightPlane`) 0 _output_get)
  (if (`self.On?`)
    (`MaterialInstanceDynamic.SetScalarParameterValue` (`self.LightMaterial`) "Intensity" (`self.Intensity`))))

(event `self.ReceiveTick`
  (params (DeltaSeconds :type "Float (single-precision)"))
  (bind _output_get (set `self.Time` (+ (`self.Time`) DeltaSeconds)))
  (if (> _output_get (`self.TurnOnAfter`))
    (`MaterialInstanceDynamic.SetScalarParameterValue` (`self.LightMaterial`) "Intensity" (`self.Intensity`))
    (`LightComponent.SetIntensity` (`self.RectLight`) 5000.0)))

(fn `UserConstructionScript`)