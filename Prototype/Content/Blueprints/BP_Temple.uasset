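; Temple actor that reacts to the player completing melodies, first lighting the temple and later opening its door.
; On BeginPlay it binds to OnAllMelodiesSung on all BP_FixedMelody actors; the first completion activates TempleLights, then swaps the binding to door opening.
; A later completion near TempleDoor removes the melody widget, plays a theme, opens the door after short delays, then unbinds and destroys a BP_FixedMelody.
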(event `SearchMelodyActor`
  (bind _outactors (`GameplayStatics.GetAllActorsOfClass` "/Game/Blueprints/Audio/AudioAnalysis/BP_FixedMelody.BP_FixedMelody_C"))
  (add `/Game/Blueprints/Audio/AudioAnalysis/BP_FixedMelody.OnAllMelodiesSung` _outactors (delegate `OnActivateLights`)))

(event `self.ReceiveBeginPlay`
  (`self.SearchMelodyActor`))

(event `OnActivateLights`
  ;[1 1 1] Activate Lighst from the Temple
  (`|ExecutionSequence`
    (:`then_0`
      (for _array_element (`self.TempleLights`)
        (`/Game/Blueprints/Art/BP_Light.OnActivateLights` _array_element)))
    (:`then_1`
      (remove `/Game/Blueprints/Audio/AudioAnalysis/BP_FixedMelody.OnAllMelodiesSung` (stale `SearchMelodyActor` _outactors) (delegate `OnActivateLights`))
      (add `/Game/Blueprints/Audio/AudioAnalysis/BP_FixedMelody.OnAllMelodiesSung` (stale `SearchMelodyActor` _outactors) (delegate `OnOpenDoor`)))))

(event `OnOpenDoor`
  (bind _templedoor (`self.TempleDoor`))
  ;[1 1 1] Open Door and play song
  (if (`/Game/Blueprints/BP_Door.IsCloseToDoor` _templedoor)
    (`KismetSystemLibrary.Delay` 1.0)
    (bind _returnvalue (`GameplayStatics.GetActorOfClass` "/Game/Blueprints/Audio/AudioAnalysis/BP_FixedMelody.BP_FixedMelody_C"))
    (`/Game/Blueprints/Audio/AudioAnalysis/BP_FixedMelody.OnRemoveMelodyWidget` _returnvalue)
    (`GameplayStatics.PlaySound2D` "/Game/Audio/wav/Cut_Theme_Temporal.Cut_Theme_Temporal" 1.0 1.0 0.0 null null)
    (`KismetSystemLibrary.Delay` 2.5)
    (`/Game/Blueprints/BP_Door.SetOpenDoor` _templedoor)
    (remove `/Game/Blueprints/Audio/AudioAnalysis/BP_FixedMelody.OnAllMelodiesSung` (stale `SearchMelodyActor` _outactors) (delegate `OnOpenDoor`))
    (`self.K2_DestroyActor` _returnvalue)))

(fn `UserConstructionScript`)