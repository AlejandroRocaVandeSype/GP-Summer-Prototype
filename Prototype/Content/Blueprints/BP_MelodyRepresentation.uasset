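; BP_MelodyRepresentation shows a target melody on screen and tracks the player's progress through it by detected pitch.
; On BeginPlay it binds to the Pitch detector and fills a UMG_Melody widget with color-coded notes.
; Pitch updates within one semitone of the current note accumulate hold time and drive that note's progress until HoldTime advances the melody.
; A note-end event resets the hold timer.
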(event `self.ReceiveBeginPlay`
  (bind _colors (`/Game/Blueprints/BP_PitchDetection.Colors` (`self.Pitch`)))
  (add `/Game/Blueprints/BP_PitchDetection.OnPitchDetectionUpdate` (`self.Pitch`) (delegate `PitchUpdate`))
  (add `/Game/Blueprints/BP_PitchDetection.NoteEnd` (`self.Pitch`) (delegate `NoteEnd`))
  (bind _returnvalue (`|CreateWidget` "/Game/ArtAssets/UI/UMG_Melody.UMG_Melody_C"))
  (bind _output_get (set `self.MelodyWidget` _returnvalue))
  (`UserWidget.AddToViewport` _output_get 0)
  (for (_array_element _array_index) (`self.Melody`)
    (`/Game/ArtAssets/UI/UMG_Melody.AddNote` _output_get (`KismetMathLibrary.Conv_ByteToInt` _array_element) (select `EMusicalNoteName` _array_element :`C` (`|GetArrayItem` _colors) :`Db` (`|GetArrayItem` _colors 1) :`D` (`|GetArrayItem` _colors 2) :`Eb` (`|GetArrayItem` _colors 3) :`E` (`|GetArrayItem` _colors 4) :`F` (`|GetArrayItem` _colors 5) :`Gb` (`|GetArrayItem` _colors 6) :`G` (`|GetArrayItem` _colors 7) :`Ab` (`|GetArrayItem` _colors 8) :`A` (`|GetArrayItem` _colors 9) :`Bb` (`|GetArrayItem` _colors 10) :`B` (`|GetArrayItem` _colors 11)) _array_element _array_index)))

(event `NoteEnd`
  (set `self.TimeNoteHeld` 0.0))

(event `PitchUpdate`
  (params (CurrentNote :type "EMusicalNoteName Enum" :default "C"))
  (bind _returnvalue (`KismetMathLibrary.Conv_ByteToInt` CurrentNote))
  (bind _returnvalue_2 (`KismetMathLibrary.Conv_ByteToInt` (`|GetArrayItem` (`self.Melody`) (`self.CurrentNote`))))
  (if (< (`self.CurrentNote`) (`KismetArrayLibrary.Array_Length` (`self.Melody`)))
    (if (or (== _returnvalue _returnvalue_2) (== (+ _returnvalue 1) _returnvalue_2) (== (+ _returnvalue -1) _returnvalue_2))
      (bind _output_get (set `self.TimeNoteHeld` (+ (`self.TimeNoteHeld`) (`GameplayStatics.GetWorldDeltaSeconds`))))
      (`KismetSystemLibrary.PrintString` (`KismetStringLibrary.Conv_DoubleToString` _output_get) true true (struct :`R` 1.0 :`G` 0.5852 :`A` 1.0))
      (if (>= (`self.TimeNoteHeld`) (`self.HoldTime`))
        (`/Engine/EditorBlueprintResources/StandardMacros.IncrementInt` (`self.CurrentNote`)
          (:`  `
            (set `self.TimeNoteHeld` 0.0)))
        (else
          (`/Game/ArtAssets/UI/UMG_Note.SetProgress` (`|GetArrayItem` (`/Game/ArtAssets/UI/UMG_Melody.Notes` (`self.MelodyWidget`)) (`self.CurrentNote`)) (/ (`self.TimeNoteHeld`) (`self.HoldTime`))))))))

(fn `UserConstructionScript`)