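; A singable note on a chord wall that lights up when the player sings its pitch.
; It finds the voice pitch analyzer and chord wall at BeginPlay and listens for pitch changes.
; When its chord is current and the sung note matches, it fires a correctly-sung event and, the first time, a discovered event.
; A timeline then blends the mesh from grey to the detector's color for that note; undiscovered notes stay dark.
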(event `self.ReceiveBeginPlay`
  (bind _returnvalue (`GameplayStatics.GetActorOfClass` "/Game/Blueprints/Audio/AudioAnalysis/BP_VoicePitchAnalyzer.BP_VoicePitchAnalyzer_C"))
  (`/Engine/EditorBlueprintResources/StandardMacros.IsValid` _returnvalue
    (:`Is Valid`
      (set `self.VoicePitchData` _returnvalue)
      (bind _returnvalue_2 (`GameplayStatics.GetActorOfClass` "/Game/Blueprints/BP_ChordWall.BP_ChordWall_C"))
      (set `self.ChordWall` _returnvalue_2)
      (add `/Game/Blueprints/Audio/AudioAnalysis/BP_VoicePitchAnalyzer.OnVoicePitchChange` (`self.VoicePitchData`) (delegate `OnVoicePitchChange_Event`))
      (`self.SetNoteColor` 1.0))
    (:`Is Not Valid`
      (`KismetSystemLibrary.PrintString` "No VoicePitchData blueprint found in scene" true true (struct :`R` 1.0 :`G` 0.014424 :`A` 1.0)))))

(event `OnVoicePitchChange_Event`
  (params (NoteNumber :type Integer) (NoteName :type "EMusicalNoteName Enum" :default "C") (NoteColor :type "LinearColor Structure"))
  (bind _chordwall (`self.ChordWall`))
  ;[1 1 1] Check if we're singing this note
  (`/Engine/EditorBlueprintResources/StandardMacros.IsValid` _chordwall
    (:`Is Valid`
      (if (== (`/Game/Blueprints/BP_ChordWall.CurrentChord` _chordwall) (`self.ChordIndex`))
        ;[1 1 1] Is the player singing the right pitch for this note?
        (if (`|EnumEquality` NoteName (`self.MusicalNote`))
          (`self.OnNoteCorrectlySung` (`self.NoteIndex`))
          ;[1 1 1] Yes: Color the note
          (`self.NoteDiscovered`)
          (bind (_direction _notediscovered) (`Timeline|Timeline`)
            (:`Update`
              (`self.SetNoteColor` _notediscovered))))))
    (:`Is Not Valid`
      (`KismetSystemLibrary.PrintString` "Chordwall not valid"))))

(fn `NoteDiscovered`
  (if (not (`self.IsDiscovered`))
    (set `self.IsDiscovered` true)
    (`self.OnNoteDiscovered` (`self.NoteIndex`))))

(fn `SetNoteColor`
  (params (LerpAlpha :type "Float (double-precision)"))
  (bind _notecolors (`/Game/Blueprints/Audio/AudioAnalysis/BPC_PitchDetector.NoteColors` (`/Game/Blueprints/Audio/AudioAnalysis/BP_VoicePitchAnalyzer.BPC_PitchDetector` (`self.VoicePitchData`))))
  (if (`self.IsDiscovered`)
    (`MeshComponent.SetVectorParameterValueOnMaterials` (`self.NoteMesh`) "Color" (`KismetMathLibrary.Conv_LinearColorToVector` (`KismetMathLibrary.LinearColorLerp` (struct :`R` 0.5 :`G` 0.5 :`B` 0.5 :`A` 1.0) (select `EMusicalNoteName` (`self.MusicalNote`) :`C` (`|GetArrayItem` _notecolors) :`Db` (`|GetArrayItem` _notecolors 1) :`D` (`|GetArrayItem` _notecolors 2) :`Eb` (`|GetArrayItem` _notecolors 3) :`E` (`|GetArrayItem` _notecolors 4) :`F` (`|GetArrayItem` _notecolors 5) :`Gb` (`|GetArrayItem` _notecolors 6) :`G` (`|GetArrayItem` _notecolors 7) :`Ab` (`|GetArrayItem` _notecolors 8) :`A` (`|GetArrayItem` _notecolors 9) :`Bb` (`|GetArrayItem` _notecolors 10) :`B` (`|GetArrayItem` _notecolors 11)) LerpAlpha)))
    (else
      (`MeshComponent.SetVectorParameterValueOnMaterials` (`self.NoteMesh`) "Color" (0.1 0.1 0.1)))))

(fn `UserConstructionScript`)