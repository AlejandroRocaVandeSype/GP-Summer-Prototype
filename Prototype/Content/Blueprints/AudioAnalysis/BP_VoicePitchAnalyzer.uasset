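; Voice pitch analyzer Blueprint that surfaces live pitch and volume data as on-screen debug text.
; It watches the "volume" output of the MSVoice MetaSound through the MetaSound Output Subsystem and prints each change.
; BPC_PitchDetector pitch updates, noted as firing above a volume threshold, store the note number, name and color.
; Tick prints the stored note every frame, tinted with its color.
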(event `self.ReceiveBeginPlay`
  ;[0.06727 1 0] Initialising metasound data stream
  (`MetaSoundOutputSubsystem.WatchOutput` (subsystem `MetaSoundOutputSubsystem`) (`self.MS_Voice`) "volume" (delegate `VolumeChange`) "None" "None"))

(event `VolumeChange`
  (params (OutputName :type Name) (Output :type "MetaSoundOutput Structure (by ref)"))
  ;[0.06727 1 0] Initialising metasound data stream
  (bind (_success _returnvalue) (`MetasoundOutputBlueprintAccess.GetFloat` Output))
  (`KismetSystemLibrary.PrintString` (`KismetStringLibrary.Conv_DoubleToString` _returnvalue) false true (struct :`R` 1.0 :`G` 0.040901 :`A` 1.0)))

(event `self.BPC_PitchDetector.OnPitchUpdate`
  (params (NoteNumber :type Integer) (NoteName :type "EMusicalNoteName Enum" :default "C") (NoteColor :type "LinearColor Structure"))
  ;[1 0.2448 0.1851] Getting pitch data when volume threshold is exceeded
  (set `self.Note Number` NoteNumber)
  (set `self.Note Name` NoteName)
  (set `self.Note Color` NoteColor))

(event `self.ReceiveTick`
  (params (DeltaSeconds :type "Float (single-precision)"))
  ;[0 0 0] Debug info
  (`KismetSystemLibrary.PrintString` (`KismetTextLibrary.Conv_TextToString` (`|FormatText` "Voice Pitch Data \nNote number: {a} \nNote Name: {b}" (`self.Note Number`) (`|GetEnumeratorNameAsString` (`self.Note Name`)))) true false (`self.Note Color`) DeltaSeconds))

(fn `UserConstructionScript`)