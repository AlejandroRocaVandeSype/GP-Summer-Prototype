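; Voice pitch analyzer that reports the note the player sings and when voice input ends.
; Relays BPC_PitchDetector events through its own dispatchers, passing note number, name and color only while BP_FPCharacter is singing.
; Exposes a setter for the detector's volume threshold and prints the current note every tick for debugging.
; Also watches the MSVoice MetaSound volume output, though that value goes unused.
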(event `self.ReceiveBeginPlay`
  ;[0.06727 1 0] Initialising metasound data stream
  (`MetaSoundOutputSubsystem.WatchOutput` (subsystem `MetaSoundOutputSubsystem`) (`self.MS_Voice`) "volume" (delegate `VolumeChange`) "None" "None")
  (bind _returnvalue (`GameplayStatics.GetActorOfClass` "/Game/Blueprints/Character/BP_FPCharacter.BP_FPCharacter_C"))
  (set `self.Player` _returnvalue))

(event `VolumeChange`
  (params (OutputName :type Name) (Output :type "MetaSoundOutput Structure (by ref)"))
  ;[0.06727 1 0] Initialising metasound data stream
  (`MetasoundOutputBlueprintAccess.GetFloat` Output))

(event `self.BPC_PitchDetector.OnPitchUpdate`
  (params (NoteNumber :type Integer) (NoteName :type "EMusicalNoteName Enum" :default "C") (NoteColor :type "LinearColor Structure"))
  ;[1 0.2448 0.1851] Getting pitch data when volume threshold is exceeded
  (if (`FPCharacter.IsPlayerSinging` (`self.Player`))
    (set `self.Note Number` NoteNumber)
    (set `self.Note Name` NoteName)
    (set `self.Note Color` NoteColor)
    (`self.OnVoicePitchChange` (`self.Note Number`) (`self.Note Name`) (`self.Note Color`))))

(event `self.BPC_PitchDetector.OnNoteEnd`
  ;[1 0.7171 0.2353] Broadcasting when no input is detected
  (`self.OnVoiceInputEnd`))

(event `self.ReceiveTick`
  (params (DeltaSeconds :type "Float (single-precision)"))
  ;[0 0 0] Debug info
  (`KismetSystemLibrary.PrintString` (`KismetTextLibrary.Conv_TextToString` (`|FormatText` "Voice Pitch Data \nNote number: {a} \nNote Name: {b}" (`self.Note Number`) (`|GetEnumeratorNameAsString` (`self.Note Name`)))) true false (`self.Note Color`) DeltaSeconds))

(fn `UpdateVolumeThreshold`
  (params (NewThreshold :type "Float (double-precision)"))
  (bind _output_get (set `/Game/Blueprints/Audio/AudioAnalysis/BPC_PitchDetector.VolumeThreshold` NewThreshold (`self.BPC_PitchDetector`))))

(fn `UserConstructionScript`)