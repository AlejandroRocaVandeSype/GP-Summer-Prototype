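; BP_AudioCapture is an actor that toggles microphone capture based on whether the first-person player character is singing.
; Every tick it casts the player character to BP_FPCharacter and starts or stops its AudioCapture component from the IsPlayerSinging flag.
; The envelope-value event is bound but does nothing, with only a disconnected debug print left beside it.
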(event `self.ReceiveBeginPlay`)

(event `self.ReceiveTick`
  (params (DeltaSeconds :type "Float (single-precision)"))
  (bind _audiocapture (`self.AudioCapture`))
  (bind _asbp_fpcharacter (cast `/Game/Blueprints/Character/BP_FPCharacter` (`GameplayStatics.GetPlayerCharacter` 0)))
  (if (`KismetSystemLibrary.IsValid` _asbp_fpcharacter)
    (if (`FPCharacter.IsPlayerSinging` _asbp_fpcharacter)
      (`SynthComponent.Start` _audiocapture)
      (else
        (`SynthComponent.Stop` _audiocapture)))))

(event `self.AudioCapture.OnAudioEnvelopeValue`
  (params (EnvelopeValue :type "Float (single-precision)")))

(fn `UserConstructionScript`)