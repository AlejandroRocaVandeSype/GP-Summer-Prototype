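; BP_MelodyButton is a button actor that plays a 2D theme sound when pressed and shows a pressed material.
; OnButtonPressed ignores presses while IsMelodyPlaying is set.
; Tick clears that flag after a fixed five-second Delay, independent of the sound's actual length, and otherwise reapplies the not-pressed material every frame.
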(event `OnButtonPressed`
  (if (not (`self.IsMelodyPlaying`))
    (`GameplayStatics.PlaySound2D` "/Game/Audio/wav/Cut_Theme_Temporal.Cut_Theme_Temporal" 1.0 1.0 0.0 null null)
    (set `self.IsMelodyPlaying` true)
    (`PrimitiveComponent.SetMaterial` (`self.Button`) 0 "/Game/ArtAssets/Materials/MI_ButtonPressed.MI_ButtonPressed")))

(event `self.ReceiveTick`
  (params (DeltaSeconds :type "Float (single-precision)"))
  (if (`self.IsMelodyPlaying`)
    (`KismetSystemLibrary.Delay` 5.0)
    (set `self.IsMelodyPlaying` false)
    (else
      (`PrimitiveComponent.SetMaterial` (`self.Button`) 0 "/Game/ArtAssets/Materials/MI_ButtonNotPressed.MI_ButtonNotPressed"))))

(fn `UserConstructionScript`)