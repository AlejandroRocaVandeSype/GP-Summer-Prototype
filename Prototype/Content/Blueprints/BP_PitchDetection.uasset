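; Detects the dominant musical note in an audio submix, colours a Niagara effect by that note and notifies of pitch updates.
; Musical-band spectral analysis runs at BeginPlay, and the loudest band's index yields note, octave and MIDI number.
; Magnitudes reaching VolumeThreshold fire the pitch update, otherwise note end is called.
; A watched MetaSound volume output and per-tick note readout only feed debug prints.
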(event `self.ReceiveBeginPlay`
  (`MetaSoundOutputSubsystem.WatchOutput` (subsystem `MetaSoundOutputSubsystem`) null "volume" (delegate `InputDetected`) "None" "None")
  (`SoundSubmix.AddSpectralAnalysisDelegate` (`self.SubmixToAnalyse`) (`AudioMixerBlueprintLibrary.MakeMusicalSpectralAnalysisBandSettings` 60 "C" (`self.StartingOctave`) 5 250) (delegate `AnalyseSubmix`) 30.0 -40.0 true true 0.1 60.0)
  (`SoundSubmix.StartSpectralAnalysis` (`self.SubmixToAnalyse`) "Max" "Quadratic" "Hann" 0.0 "Decibel"))

(event `InputDetected`
  (params (OutputName :type Name) (Output :type "MetaSoundOutput Structure (by ref)"))
  (bind (_success _returnvalue) (`MetasoundOutputBlueprintAccess.GetFloat` Output))
  (bind _output_get (set `self.CurrentAmplitude` _returnvalue))
  (`KismetSystemLibrary.PrintString` (`KismetStringLibrary.Conv_DoubleToString` _output_get) true true (struct :`R` 1.0 :`G` 0.040901 :`A` 1.0)))

(event `AnalyseSubmix`
  (params (Magnitude :type "Array of Float (single-precision) (by ref)"))
  (bind (_indexofmaxvalue _maxvalue) (`KismetMathLibrary.MaxOfFloatArray` Magnitude))
  (set `self.CurrentNoteMagnitude` _maxvalue)
  (set `self.CurrentNoteNumber` (mod _indexofmaxvalue 12))
  (set `self.CurrentOctave` (/ _indexofmaxvalue 12))
  (set `self.CurrentMIDINote` (+ (`self.CurrentNoteNumber`) (* (+ (`self.CurrentOctave`) 2) 12)))
  (set `self.CurentNoteName` (select `int` (`self.CurrentNoteNumber`) :`0` "C" :`1` "Db" :`2` "D" :`3` "Eb" :`4` "E" :`5` "F" :`6` "Gb" :`7` "G" :`8` "Ab" :`9` "A" :`10` "Bb" :`11` "B" :!type "EMusicalNoteName Enum"))
  (set `self.CurrentColor` (`|GetArrayItem` (`self.Colors`) (`self.CurrentNoteNumber`)))
  (`self.UpdateNiagaraSystem`)
  (if (>= (`self.CurrentNoteMagnitude`) (`self.VolumeThreshold`))
    (`self.PitchDetectUpdate`)
    (else
      (`self.NoteEnd`))))

(event `self.ReceiveTick`
  (params (DeltaSeconds :type "Float (single-precision)"))
  ;[1 1 1] Debug info
  (`KismetSystemLibrary.PrintString` (`KismetTextLibrary.Conv_TextToString` (`|FormatText` "Spectral Data \nNote number: {a} \nNote Name: {b} \nAmplitude \nOutput volume: {e}" (`self.CurrentNoteNumber`) (`|GetEnumeratorNameAsString` (`self.CurentNoteName`)) (`self.CurrentNoteMagnitude`))) true true (`self.CurrentColor`) DeltaSeconds))

(event `UpdateNiagaraSystem`
  (`NiagaraComponent.SetVariableLinearColor` (`self.Niagara`) "NoteColor" (`self.CurrentColor`)))

(event `PitchDetectUpdate`
  (`self.OnPitchDetectionUpdate` (`self.CurentNoteName`)))

(fn `UserConstructionScript`)