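; Pitch detector component that finds the dominant musical note in an audio submix and broadcasts it with a name and colour.
; On BeginPlay it starts spectral analysis using semitone-spaced bands.
; Each update takes the loudest band modulo 12 as the pitch class, assuming the strongest band is the fundamental.
; Above the volume threshold it calls OnPitchUpdate, otherwise it calls OnNoteEnd on every update.
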(event `self.ReceiveBeginPlay`
  ;[0 1 0.004799] Initialising submix analysis
  ;;[1 1 1] Creating Spectral Analysis Delegate
  (`SoundSubmix.AddSpectralAnalysisDelegate` (`self.SubmixToAnalyse`) (`AudioMixerBlueprintLibrary.MakeMusicalSpectralAnalysisBandSettings` (`self.NrOfSemiTones`) "C" (`self.StartingOctave`) 5 250) (delegate `OnSpectralAnalysis`) 30.0 -40.0 true true 0.1 60.0)
  ;;[1 1 1] Starting analysis
  (`SoundSubmix.StartSpectralAnalysis` (`self.SubmixToAnalyse`) "Max" "Quadratic" "Hann" 0.0 "Decibel"))

(event `OnSpectralAnalysis`
  (params (Magnitude :type "Array of Float (single-precision) (by ref)"))
  (bind (_indexofmaxvalue _maxvalue) (`KismetMathLibrary.MaxOfFloatArray` Magnitude))
  ;[0 0.9234 1] Updating pitch detection data
  ;;[1 1 1] Getting fundamental frequency from spectral analysis data
  (set `self.CurrentNoteMagnitude` _maxvalue)
  ;;[1 1 1] Checking if volume threshold is exceeded
  (if (>= (`self.CurrentNoteMagnitude`) (`self.VolumeThreshold`))
    ;;[1 1 1] Updating pitch parameter if volume threshold is exceeded
    ;;;[1 1 1] Calculating current note number
    (set `self.CurrentNoteNumber` (mod _indexofmaxvalue 12))
    ;;;[1 1 1] Getting current note name
    (set `self.CurentNoteName` (select `int` (`self.CurrentNoteNumber`) :`0` "C" :`1` "Db" :`2` "D" :`3` "Eb" :`4` "E" :`5` "F" :`6` "Gb" :`7` "G" :`8` "Ab" :`9` "A" :`10` "Bb" :`11` "B" :!type "EMusicalNoteName Enum"))
    ;;;[1 1 1] Getting colour associated with note number
    (set `self.CurrentNoteColor` (`|GetArrayItem` (`self.NoteColors`) (`self.CurrentNoteNumber`)))
    (`self.OnPitchUpdate` (`self.CurrentNoteNumber`) (`self.CurentNoteName`) (`self.CurrentNoteColor`))
    (else
      (`self.OnNoteEnd`))))