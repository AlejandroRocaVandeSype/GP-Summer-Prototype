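; Fixed-melody singing minigame Blueprint, where the player sings a preset sequence of notes in order.
; On BeginPlay it binds to VoicePitchData events and builds a UMG melody widget, colouring each note from the pitch detector's palette.
; Pitch changes update the current-note indicator and, within one semitone of the target, accumulate hold time to show progress and advance the melody.
; Voice input ending resets the hold timer.
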(event `self.ReceiveBeginPlay`
  (bind _notecolors (`/Game/Blueprints/AudioAnalysis/BPC_PitchDetector.NoteColors` (`/Game/Blueprints/AudioAnalysis/BP_VoicePitchAnalyzer.BPC_PitchDetector` (`self.VoicePitchData`))))
  ;[0 1 0.09038] Initialising fixed melody minigame
  ;;[1 1 1] Binding voice pitch data events
  (add `/Game/Blueprints/AudioAnalysis/BP_VoicePitchAnalyzer.OnVoicePitchChange` (`self.VoicePitchData`) (delegate `VoicePitchChange`))
  (add `/Game/Blueprints/AudioAnalysis/BP_VoicePitchAnalyzer.OnVoiceInputEnd` (`self.VoicePitchData`) (delegate `ResetTimeNoteHeld`))
  ;;[1 1 1] Creating melody widget
  (bind _returnvalue (`|CreateWidget` "/Game/ArtAssets/UI/UMG_Melody.UMG_Melody_C"))
  (bind _output_get (set `self.MelodyWidget` _returnvalue))
  (`UserWidget.AddToViewport` _output_get 0)
  ;;[1 1 1] Initialising melody widget with correct notes based on melody array
  (for (_array_element _array_index) (`self.Melody`)
    (`/Game/ArtAssets/UI/UMG_Melody.AddNote` _output_get (`KismetMathLibrary.Conv_ByteToInt` _array_element) (select `EMusicalNoteName` _array_element :`C` (`|GetArrayItem` _notecolors) :`Db` (`|GetArrayItem` _notecolors 1) :`D` (`|GetArrayItem` _notecolors 2) :`Eb` (`|GetArrayItem` _notecolors 3) :`E` (`|GetArrayItem` _notecolors 4) :`F` (`|GetArrayItem` _notecolors 5) :`Gb` (`|GetArrayItem` _notecolors 6) :`G` (`|GetArrayItem` _notecolors 7) :`Ab` (`|GetArrayItem` _notecolors 8) :`A` (`|GetArrayItem` _notecolors 9) :`Bb` (`|GetArrayItem` _notecolors 10) :`B` (`|GetArrayItem` _notecolors 11)) _array_element _array_index)))

(event `ResetTimeNoteHeld`
  ;[1 0.5418 0.2977] Resetting time note held
  (set `self.TimeNoteHeld` 0.0))

(event `VoicePitchChange`
  (params (NoteNumber :type Integer) (NoteName :type "EMusicalNoteName Enum" :default "C") (NoteColor :type "LinearColor Structure"))
  (bind _returnvalue (`KismetMathLibrary.Conv_ByteToInt` NoteName))
  (bind _returnvalue_2 (`KismetMathLibrary.Conv_ByteToInt` (`|GetArrayItem` (`self.Melody`) (`self.CurrentNote`))))
  ;[1 0.8357 0.1739] Updating melody widget on voice pitch change
  (`|ExecutionSequence`
    (:`then_0`
      ;;[1 1 1] Updating melody widget current note indicator
      (`/Game/ArtAssets/UI/UMG_CurrentNote.UpdateCurrentNote` (`/Game/ArtAssets/UI/UMG_Melody.UMG_CurrentNote` (`self.MelodyWidget`)) NoteName))
    (:`then_1`
      ;;[1 1 1] Check if current note is in range of melody
      (if (< (`self.CurrentNote`) (`KismetArrayLibrary.Array_Length` (`self.Melody`)))
        ;;[1 1 1] Check if note currently being sung is correct, with a margin of -1/+1 semitone
        (if (or (== _returnvalue _returnvalue_2) (== (+ _returnvalue 1) _returnvalue_2) (== (+ _returnvalue -1) _returnvalue_2))
          ;;[1 1 1] Increase time note held
          (set `self.TimeNoteHeld` (+ (`self.TimeNoteHeld`) (`GameplayStatics.GetWorldDeltaSeconds`)))
          ;;[1 1 1] Check if note has been held long enough
          (if (>= (`self.TimeNoteHeld`) (`self.HoldTime`))
            ;;[1 1 1] Go to next note in melody and reset time held
            (`/Engine/EditorBlueprintResources/StandardMacros.IncrementInt` (`self.CurrentNote`)
              (:`  `
                (set `self.TimeNoteHeld` 0.0)))
            (else
              ;;[1 1 1] Update note visual
              (`/Game/ArtAssets/UI/UMG_Note.SetProgress` (`|GetArrayItem` (`/Game/ArtAssets/UI/UMG_Melody.Notes` (`self.MelodyWidget`)) (`self.CurrentNote`)) (/ (`self.TimeNoteHeld`) (`self.HoldTime`))))))))))

(fn `UserConstructionScript`)