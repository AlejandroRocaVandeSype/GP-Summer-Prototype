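; Fixed melody singing minigame that has the player sing a set sequence of notes, tracked in a UMG_FixedMelody widget.
; Pitch events from BP_VoicePitchAnalyzer advance the melody when a note within one semitone is held for HoldTime; input end resets the timer.
; AddMelodyNotes extends the melody and can show the widget, which colors notes from the pitch detector palette.
; Completion fires AllMelodiesSung, then optionally hides the widget or resets progress.
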(event `self.ReceiveBeginPlay`
  ;[1 1 1] Create the widget but dont add it to the HUD yet
  (bind _returnvalue (`|CreateWidget` "/Game/Blueprints/UI/UMG_FixedMelody.UMG_FixedMelody_C"))
  (set `self.MelodyWidget` _returnvalue)
  ;[1 1 1] Setup the Voice Pitch Data Actor
  (`/Engine/EditorBlueprintResources/StandardMacros.IsValid` (`self.VoicePitchData`)
    (:`Is Valid`
      _)
    (:`Is Not Valid`
      (`self.Init Voice Pitch Data`)))
  ;[0 1 0.09038] Initialising fixed melody minigame
  ;;[1 1 1] Binding voice pitch data events
  (add `/Game/Blueprints/Audio/AudioAnalysis/BP_VoicePitchAnalyzer.OnVoicePitchChange` (`self.VoicePitchData`) (delegate `VoicePitchChange`))
  (add `/Game/Blueprints/Audio/AudioAnalysis/BP_VoicePitchAnalyzer.OnVoiceInputEnd` (`self.VoicePitchData`) (delegate `ResetTimeNoteHeld`))
  (if (> (`KismetArrayLibrary.Array_Length` (`self.Melody`)) 0)
    (`self.InitMelody`)))

(event `OnRemoveMelodyWidget`
  ;[1 1 1] Add / Remove the FixedMelody WIdget from HUD
  (if (`self.IsOnWidget`)
    (set `self.IsOnWidget` false)
    (`Widget.RemoveFromParent` (`self.MelodyWidget`))))

(event `ResetTimeNoteHeld`
  ;[1 0.5418 0.2977] Resetting time note held
  (set `self.TimeNoteHeld` 0.0))

(event `OnAddMelodyWidget`
  ;[1 1 1] Add / Remove the FixedMelody WIdget from HUD
  (if (not (`self.IsOnWidget`))
    (`UserWidget.AddToViewport` (`self.MelodyWidget`) 0)
    (set `self.IsOnWidget` true)))

(event `VoicePitchChange`
  (params (NoteNumber :type Integer) (NoteName :type "EMusicalNoteName Enum" :default "C") (NoteColor :type "LinearColor Structure"))
  (bind _returnvalue (`KismetMathLibrary.Conv_ByteToInt` NoteName))
  (bind _melodiessang (`self.MelodiesSang`))
  (bind _currentnote (`self.CurrentNote`))
  (bind _returnvalue_2 (`KismetMathLibrary.Conv_ByteToInt` (`|GetArrayItem` (`self.Melody`) (`self.CurrentNote`))))
  ;[1 0.8357 0.1739] Updating melody widget on voice pitch change
  (`|ExecutionSequence`
    (:`then_0`
      ;;[1 1 1] Updating melody widget current note indicator
      (`/Game/Blueprints/UI/UMG_CurrentNote.UpdateCurrentNote` (`/Game/Blueprints/UI/UMG_FixedMelody.UMG_CurrentNote` (`self.MelodyWidget`)) NoteName))
    (:`then_1`
      ;;[1 1 1] Check if current note is in range of melody
      (if (< (`self.CurrentNote`) (`KismetArrayLibrary.Array_Length` (`self.Melody`)))
        ;;[1 1 1] Check if note currently being sung is correct, with a margin of -1/+1 semitone
        (if (or (== _returnvalue _returnvalue_2) (== (+ _returnvalue 1) _returnvalue_2) (== (+ _returnvalue -1) _returnvalue_2))
          ;;[1 1 1] Increase time note held
          (set `self.TimeNoteHeld` (+ (`self.TimeNoteHeld`) (`GameplayStatics.GetWorldDeltaSeconds`)))
          ;;[1 1 1] Check if note has been held long enough
          (if (>= (`self.TimeNoteHeld`) (`self.HoldTime`))
            ;;[1 1 1] Go to next note in melody and reset time held
            (`/Engine/EditorBlueprintResources/StandardMacros.IncrementInt` (`self.CurrentNote`)
              (:`  `
                (set `self.TimeNoteHeld` 0.0)
                ;;[1 1 1] Check if there are still melodies to sing
                (bind _result (`/Engine/EditorBlueprintResources/StandardMacros.IncrementInt` _melodiessang)
                  (:`  `
                    (`KismetSystemLibrary.PrintString` (`KismetStringLibrary.Conv_IntToString` _melodiessang))
                    (if (== _result (`self.TotalNrMelodies`))
                      ;[1 0.3514 0.06186] All melodies have been sung
                      (`self.OnAllMelodiesSung`)
                      (`|ExecutionSequence`
                        (:`then_0`
                          ;;[1 1 1] Check if the Melody Widget needs to be removed from the HUD
                          (if (`self.DoRemoveFromWidget`)
                            (`KismetSystemLibrary.Delay` 1.0)
                            (`self.OnRemoveMelodyWidget`)))
                        (:`then_1`
                          ;;[1 1 1] Check if the Melody Info needs to be reset
                          (if (`self.DoResetMelody`)
                            (set `self.MelodiesSang` 0)
                            (set `self.CurrentNote` 0)
                            (while (< _currentnote (`self.TotalNrMelodies`))
                              (`/Game/Blueprints/UI/UMG_Note.ResetProgress` (`|GetArrayItem` (`/Game/Blueprints/UI/UMG_FixedMelody.Notes` (`self.MelodyWidget`)) _currentnote))
                              (bind _result_2 (`/Engine/EditorBlueprintResources/StandardMacros.IncrementInt` _currentnote)
                                (:`  `
                                  (set `self.CurrentNote` _result_2))))
                            (set `self.CurrentNote` 0)))))))))
            (else
              ;;[1 1 1] Update note visual
              (`/Game/Blueprints/UI/UMG_Note.SetProgress` (`|GetArrayItem` (`/Game/Blueprints/UI/UMG_FixedMelody.Notes` (`self.MelodyWidget`)) (`self.CurrentNote`)) (/ (`self.TimeNoteHeld`) (`self.HoldTime`))))))))))

(fn `Add Melody Notes`
  (params (NewMelodies :type "Array of EMusicalNoteName Enum") (ShowMelodyUI :type Boolean))
  (bind _melody (`self.Melody`))
  (for _array_element NewMelodies
    (`KismetArrayLibrary.Array_Add` _melody _array_element))
  (set `self.TotalNrMelodies` (`KismetArrayLibrary.Array_Length` _melody))
  (`self.InitMelody`)
  (if ShowMelodyUI
    (`self.OnAddMelodyWidget`)))

(fn `Add Melody Widget`
  (returns (OutputPin :type "/Game/Blueprints/UI/UMG_FixedMelody Object Reference"))
  (bind _returnvalue (`|CreateWidget` "/Game/Blueprints/UI/UMG_FixedMelody.UMG_FixedMelody_C"))
  (bind _output_get (set `self.MelodyWidget` _returnvalue))
  (`UserWidget.AddToViewport` _output_get 0)
  (return _output_get))

(fn `AddNote`
  (bind _notesadded (`self.NotesAdded`))
  (bind _output (`|GetArrayItem` (`self.Melody`) _notesadded))
  (bind _notecolors (`/Game/Blueprints/Audio/AudioAnalysis/BPC_PitchDetector.NoteColors` (`/Game/Blueprints/Audio/AudioAnalysis/BP_VoicePitchAnalyzer.BPC_PitchDetector` (`self.VoicePitchData`))))
  ;[1 1 1] Add a single note ( This is to avoid adding duplicated notes to the UI )
  (`/Game/Blueprints/UI/UMG_FixedMelody.AddNote` (`self.MelodyWidget`) (`KismetMathLibrary.Conv_ByteToInt` _output) (select `EMusicalNoteName` "C" :`C` (`|GetArrayItem` _notecolors) :`Db` (`|GetArrayItem` _notecolors 1) :`D` (`|GetArrayItem` _notecolors 2) :`Eb` (`|GetArrayItem` _notecolors 3) :`E` (`|GetArrayItem` _notecolors 4) :`F` (`|GetArrayItem` _notecolors 5) :`Gb` (`|GetArrayItem` _notecolors 6) :`G` (`|GetArrayItem` _notecolors 7) :`Ab` (`|GetArrayItem` _notecolors 8) :`A` (`|GetArrayItem` _notecolors 9) :`Bb` (`|GetArrayItem` _notecolors 10) :`B` (`|GetArrayItem` _notecolors 11)) _output _notesadded)
  (set `self.NotesAdded` (+ (`self.NotesAdded`) 1)))

(fn `Init Voice Pitch Data`
  (bind _returnvalue (`GameplayStatics.GetActorOfClass` "/Game/Blueprints/Audio/AudioAnalysis/BP_VoicePitchAnalyzer.BP_VoicePitchAnalyzer_C"))
  (`/Engine/EditorBlueprintResources/StandardMacros.IsValid` _returnvalue
    (:`Is Valid`
      (set `self.VoicePitchData` _returnvalue))
    (:`Is Not Valid`
      (`KismetSystemLibrary.PrintString` "Warning! No VoicePitchData found"))))

(fn `InitMelody`
  (bind _notecolors (`/Game/Blueprints/Audio/AudioAnalysis/BPC_PitchDetector.NoteColors` (`/Game/Blueprints/Audio/AudioAnalysis/BP_VoicePitchAnalyzer.BPC_PitchDetector` (`self.VoicePitchData`))))
  ;[1 1 1] Initialising melody widget with correct notes based on melody array ( Only once )
  (if (`self.IsMelodyInit`)
    ;[1 1 1] Add a single note ( Avoids adding the duplicated notes )
    (`self.AddNote`)
    (else
      (for (_array_element _array_index) (`self.Melody`)
        (`/Game/Blueprints/UI/UMG_FixedMelody.AddNote` (`self.MelodyWidget`) (`KismetMathLibrary.Conv_ByteToInt` _array_element) (select `EMusicalNoteName` _array_element :`C` (`|GetArrayItem` _notecolors) :`Db` (`|GetArrayItem` _notecolors 1) :`D` (`|GetArrayItem` _notecolors 2) :`Eb` (`|GetArrayItem` _notecolors 3) :`E` (`|GetArrayItem` _notecolors 4) :`F` (`|GetArrayItem` _notecolors 5) :`Gb` (`|GetArrayItem` _notecolors 6) :`G` (`|GetArrayItem` _notecolors 7) :`Ab` (`|GetArrayItem` _notecolors 8) :`A` (`|GetArrayItem` _notecolors 9) :`Bb` (`|GetArrayItem` _notecolors 10) :`B` (`|GetArrayItem` _notecolors 11)) _array_element _array_index)
        (set `self.IsMelodyInit` true)
        (set `self.NotesAdded` (+ (`self.NotesAdded`) 1))))))

(fn `UserConstructionScript`)