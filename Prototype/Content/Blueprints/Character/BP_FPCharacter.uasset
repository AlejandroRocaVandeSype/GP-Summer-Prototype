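; First-person player character Blueprint that handles item pickup, melody button presses and voice volume threshold control.
; On BeginPlay it finds the audio capture actor and creates the HUD, whose slider forwards threshold changes to the voice pitch analyzer.
; Pickup input messages overlapping items via interface, copies mesh and scale onto the equipped item, flags temple item pickups, and presses overlapping melody buttons.
; A separate input toggles the threshold slider's visibility.
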(event `self.ReceiveBeginPlay`
  (`|ExecutionSequence`
    (:`then_0`
      ;[1 1 1] Search for the Audio Capture Actor in the world
      (bind _outactors (`GameplayStatics.GetAllActorsOfClass` "/Game/Blueprints/Audio/BP_AudioCapture.BP_AudioCapture_C"))
      (bind _output (`|GetArrayItem` _outactors))
      (`/Engine/EditorBlueprintResources/StandardMacros.IsValid` _output
        (:`Is Valid`
          (set `self.AudioCapture` _output))
        (:`Is Not Valid`
          (`KismetSystemLibrary.PrintString` "Warning! Audio Capture Class not found"))))
    (:`then_1`
      ;[1 1 1] Show Player HUD
      (bind _returnvalue (`|CreateWidget` "/Game/Blueprints/UI/UMG_PlayerHUD.UMG_PlayerHUD_C"))
      (`UserWidget.AddToViewport` _returnvalue 0)
      (set `self.HUDWidget` _returnvalue)
      (add `/Game/Blueprints/UI/UMG_PlayerHUD.OnSliderValueChanged` _returnvalue (delegate `UpdateVolumeThreshold`)))))

(event `UpdateVolumeThreshold`
  (params (`Threeshold Value` :type "Float (double-precision)"))
  ;[1 1 1] Update the Volume for the Threeshold
  (bind _returnvalue (`GameplayStatics.GetActorOfClass` "/Game/Blueprints/Audio/AudioAnalysis/BP_VoicePitchAnalyzer.BP_VoicePitchAnalyzer_C"))
  (`/Game/Blueprints/Audio/AudioAnalysis/BP_VoicePitchAnalyzer.UpdateVolumeThreshold` _returnvalue `Threeshold Value`))

(event `EnhancedInput|/Game/Blueprints/Input/Actions/IA_PickupItem`
  (params (ActionValue :type Boolean) (ElapsedSeconds :type "Float (double-precision)") (TriggeredSeconds :type "Float (double-precision)") (InputAction :type "InputAction Object Reference" :default "/Game/Blueprints/Input/Actions/IA_PickupItem.IA_PickupItem"))
  (bind _equippeditem (`self.EquippedItem`))
  (:`Triggered`
    (`|ExecutionSequence`
      (:`then_0`
        ;[1 1 1] Loop over all items we're overlapping
        (for _array_element (`self.GetOverlappingActors` "/Game/Blueprints/BP_Item.BP_Item_C")
          (if (`KismetSystemLibrary.DoesImplementInterface` _array_element "/Game/Blueprints/BPI_Items.BPI_Items_C")
            (message `/Game/Blueprints/BPI_Items.Pickup` _array_element)
            (break)))
        (`|ExecutionSequence`
          (:`then_0`
            (bind _asbp_item (cast `/Game/Blueprints/BP_Item` _array_element))
            (`|ExecutionSequence`
              (:`then_0`
                (`StaticMeshComponent.SetStaticMesh` _equippeditem (`/Game/Blueprints/BP_Item.ItemMesh` _asbp_item))
                (`SceneComponent.SetWorldScale3D` _equippeditem (`self.GetActorScale3D` _asbp_item)))
              (:`then_1`
                (cast `/Game/Blueprints/BP_TempleItem` _asbp_item)
                (`self.FirstItemPickedUp`))))))
      (:`then_1`
        (for _array_element_2 (`self.GetOverlappingActors` "/Game/Blueprints/BP_MelodyButton.BP_MelodyButton_C")
          _)
        (bind _asbp_melody_button (cast `/Game/Blueprints/BP_MelodyButton` _array_element_2))
        (`/Game/Blueprints/BP_MelodyButton.OnButtonPressed` _asbp_melody_button)))))

(event `EnhancedInput|/Game/Blueprints/Input/Actions/IA_ShowThreshold`
  (params (ActionValue :type Boolean) (ElapsedSeconds :type "Float (double-precision)") (TriggeredSeconds :type "Float (double-precision)") (InputAction :type "InputAction Object Reference" :default "/Game/Blueprints/Input/Actions/IA_ShowThreshold.IA_ShowThreshold"))
  (:`Triggered`
    (`/Game/Blueprints/UI/UMG_PlayerHUD.Toggle Slider Visibility` (`self.HUDWidget`))))

(fn `UserConstructionScript`)