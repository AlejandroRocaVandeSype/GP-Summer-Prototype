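; BP_OffsetNote runs a fixed-melody voice pitch minigame where notes are sung as semitone offsets from a root the player chooses.
; On BeginPlay it builds a UMG widget from the NoteOffset array and binds to VoicePitchData events.
; Pitch changes set the root on the first step, then must match root plus offset, modulo 12.
; Matching pitches accumulate hold time to advance the melody, though the input-end reset event is empty.
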(event `self.ReceiveBeginPlay`
  (bind _noteoffset (`self.NoteOffset`))
  (`|ExecutionSequence`
    (:`then_0`
      ;[0 1 0.09038] Initialising fixed melody minigame
      ;;[1 1 1] Initialising widget
      ;;;[1 1 1] Creating melody widget
      (bind _returnvalue (`|CreateWidget` "/Game/Blueprints/UI/UMG_OffsetNote.UMG_OffsetNote_C"))
      (bind _output_get (set `self.Widget` _returnvalue))
      (`UserWidget.AddToViewport` _output_get 0)
      ;;;[1 1 1] Setting range of notes in array
      (set `/Game/Blueprints/UI/UMG_OffsetNote.MaxRows` (`KismetMathLibrary.Abs_Int` (- (`.MinValue` (`KismetMathLibrary.MinOfIntArray` _noteoffset)) (`.MaxValue` (`KismetMathLibrary.MaxOfIntArray` _noteoffset)))) (`self.Widget`))
      ;;;[1 1 1] Initialising notes
      (for (_array_element _array_index) (`self.NoteOffset`)
        (`/Game/Blueprints/UI/UMG_OffsetNote.AddNote` (`self.Widget`) _array_element (`.MinValue` (`KismetMathLibrary.MinOfIntArray` (`self.NoteOffset`))) _array_index)))
    (:`then_2`
      ;;[1 1 1] Binding voice pitch data events
      (add `/Game/Blueprints/Audio/AudioAnalysis/BP_VoicePitchAnalyzer.OnVoicePitchChange` (`self.VoicePitchData`) (delegate `VoicePitchChange`))
      (add `/Game/Blueprints/Audio/AudioAnalysis/BP_VoicePitchAnalyzer.OnVoiceInputEnd` (`self.VoicePitchData`) (delegate `ResetTimeNoteHeld`)))))

(event `ResetTimeNoteHeld`
  ;[1 0.5418 0.2977] Resetting time note held
)

(event `VoicePitchChange`
  (params (NoteNumber :type Integer) (NoteName :type "EMusicalNoteName Enum" :default "C") (NoteColor :type "LinearColor Structure"))
  (bind _returnvalue (mod (+ (`|GetArrayItem` (`self.NoteOffset`) (`self.MelodyStep`)) (`self.RootNote`)) 12))
  ;[1 0.8357 0.1739] Updating melody widget on voice pitch change
  (`|ExecutionSequence`
    (:`then_0`
      ;;[1 1 1] Updating melody widget current note indicator
      (`/Game/Blueprints/UI/UMG_CurrentNote.UpdateCurrentNote` (`/Game/Blueprints/UI/UMG_OffsetNote.UMG_CurrentNote` (`self.Widget`)) NoteName))
    (:`then_1`
      (if (== (`self.MelodyStep`) 0)
        (`/Game/Blueprints/UI/UMG_Note.SetColour` (`|GetArrayItem` (`/Game/Blueprints/UI/UMG_OffsetNote.Notes` (`self.Widget`))) NoteColor)
        (set `self.RootNote` NoteNumber)
        ;;[1 1 1] Increase time note held
        (set `self.TimeNoteHeld` (+ (`self.TimeNoteHeld`) (`GameplayStatics.GetWorldDeltaSeconds`)) :!label _label)
        ;;[1 1 1] Check if note has been held long enough
        (if (>= (`self.TimeNoteHeld`) (`self.HoldTime`))
          ;;[1 1 1] Go to next note in melody and reset time held
          (`/Engine/EditorBlueprintResources/StandardMacros.IncrementInt` (`self.MelodyStep`)
            (:`  `
              (set `self.TimeNoteHeld` 0.0)))
          (else
            ;;[1 1 1] Update note visual
            (`/Game/Blueprints/UI/UMG_Note.SetProgress` (`|GetArrayItem` (`/Game/Blueprints/UI/UMG_OffsetNote.Notes` (`self.Widget`)) (`self.MelodyStep`)) (/ (`self.TimeNoteHeld`) (`self.HoldTime`)))))
        (else
          ;;[1 1 1] Check if current note is in range of melody
          (if (< (`self.MelodyStep`) (`KismetArrayLibrary.Array_Length` (`self.NoteOffset`)))
            ;;[1 1 1] Check if current note is at the correct distance from the root
            (if (== _returnvalue NoteNumber)
              (goto _label)
              (else
                (`KismetSystemLibrary.PrintString` (`KismetTextLibrary.Conv_TextToString` (`|FormatText` "Offset that needs to be hit: {a} \nCurrent offset: {b}" _returnvalue NoteNumber)))))))))))

(fn `CreateMelodyWidget`)

(fn `UserConstructionScript`)