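; BP_TempleItem is a pickup that grants the player melody notes to sing.
; On Pickup it optionally shows the UMG_PlayerInfo widget, then passes its Notes and the ShowPickUpUI flag to the BP_FixedMelody actor found in the level.
; It destroys itself one tick later, a delay the author notes is needed to spawn the object in front of the player.
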(event `self.ReceiveBeginPlay`)

(event `/Game/Blueprints/BPI_Items.Pickup`
  (`|ExecutionSequence`
    (:`then_0`
      (`self.Pick Up Item`)
      (bind _returnvalue (`GameplayStatics.GetActorOfClass` "/Game/Blueprints/Audio/AudioAnalysis/BP_FixedMelody.BP_FixedMelody_C"))
      (`/Engine/EditorBlueprintResources/StandardMacros.IsValid` _returnvalue
        (:`Is Valid`
          (`/Game/Blueprints/Audio/AudioAnalysis/BP_FixedMelody.Add Melody Notes` _returnvalue (`self.Notes`) (`self.Show PickUp UI`)))))
    (:`then_1`
      ;[1 1 1] Need it so we can spawn the object in front of the player
      (`KismetSystemLibrary.DelayUntilNextTick`)
      (`self.K2_DestroyActor`))))

(fn `Pick Up Item`
  (`|ExecutionSequence`
    (:`then_0`
      (if (`self.Show PickUp UI`)
        ;[1 1 1] Show how to sing info on UI
        (bind _returnvalue (`|CreateWidget` "/Game/Blueprints/UI/UMG_PlayerInfo.UMG_PlayerInfo_C"))
        (`UserWidget.AddToViewport` _returnvalue 0)))))

(fn `UserConstructionScript`
  (`parent.UserConstructionScript`))