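; Enemy pawn that chases any pawn it sees and returns to its spawn point when it loses sight, using Swimming movement mode set at BeginPlay.
; PawnSensing starts an AIMoveTo toward the seen pawn and sets an in-sight flag, which a one-second retriggerable delay clears once sightings stop.
; While the flag is false, Tick reissues a move to the saved spawn location and restores capsule rotation on arrival.
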(event `self.ReceiveBeginPlay`
  (`CharacterMovementComponent.SetMovementMode` (`self.CharacterMovement`) "MOVE_Swimming" 0)
  (set `self.SpawnTransform` (`KismetMathLibrary.MakeTransform` (`self.K2_GetActorLocation`) (`self.K2_GetActorRotation`))))

(event `self.ReceiveTick`
  (params (DeltaSeconds :type "Float (single-precision)"))
  (bind _spawntransform_location (`KismetMathLibrary.BreakTransform` (`self.SpawnTransform`)))
  (bind (_spawntransform_location_2 _spawntransform_rotation) (`KismetMathLibrary.BreakTransform` (`self.SpawnTransform`)))
  (if (not (`self.IsPlayerInSight`))
    ;[1 0.9625 0.2378] Go Back to Spawn Position when Lost sight
    (`|AIMoveTo` self _spawntransform_location null
      (:`OnSuccess`
        (`SceneComponent.K2_SetRelativeRotation` (`self.CapsuleComponent`) _spawntransform_rotation false false)))))

(event `self.PawnSensing.OnSeePawn`
  (params (Pawn :type "Pawn Object Reference"))
  ;[1 1 1] AI Sight Perception
  (`|ExecutionSequence`
    (:`then_0`
      (`|AIMoveTo` self (0.0 0.0 0.0) Pawn
        (:`then`
          (set `self.IsPlayerInSight` true))))
    (:`then_1`
      (`KismetSystemLibrary.RetriggerableDelay` 1.0)
      (set `self.IsPlayerInSight` false))))

(fn `UserConstructionScript`)