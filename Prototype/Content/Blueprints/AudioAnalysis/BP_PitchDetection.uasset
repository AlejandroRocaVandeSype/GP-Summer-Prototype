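; Pitch detection Blueprint that finds the dominant musical note in a submix, likely from voice input, and broadcasts it for puzzles.
; Spectral analysis splits the audio into semitone bands; the loudest band gives note name, number, octave and color.
; Each update tints a Niagara system, then broadcasts the note if its magnitude meets a threshold, otherwise calls note end.
; Tick prints debug readouts; the MetaSound volume watcher's handler is empty.
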(event `self.ReceiveTick`
  (params (DeltaSeconds :type "Float (single-precision)"))
  ;[1 1 1] Debug info
  (`KismetSystemLibrary.PrintString` (`KismetTextLibrary.Conv_TextToString` (`|FormatText` "Spectral Data \nNote number: {a} \nNote Name: {b} \nAmplitude \nOutput volume: {e}" (`self.CurrentNoteNumber`) (`|GetEnumeratorNameAsString` (`self.CurentNoteName`)) (`self.CurrentNoteMagnitude`))) true false (`self.CurrentColor`) DeltaSeconds))

(event `self.ReceiveBeginPlay`
  ;[1 1 1] Watching MS_Voice output
  (`MetaSoundOutputSubsystem.WatchOutput` (subsystem `MetaSoundOutputSubsystem`) (`self.MS_Voice`) "volume" (delegate `InputDetected`) "None" "None")
  ;[1 1 1] Initialising submix analysis
  ;;[1 1 1] Creating Spectral Analysis Delegate
  (`SoundSubmix.AddSpectralAnalysisDelegate` (`self.SubmixToAnalyse`) (`AudioMixerBlueprintLibrary.MakeMusicalSpectralAnalysisBandSettings` 48 "C" (`self.StartingOctave`) 5 250) (delegate `AnalyseSubmix`) 30.0 -40.0 true true 0.1 60.0)
  ;;[1 1 1] Starting analysis
  (`SoundSubmix.StartSpectralAnalysis` (`self.SubmixToAnalyse`) "Max" "Quadratic" "Hann" 0.0 "Decibel"))

(event `InputDetected`
  (params (OutputName :type Name) (Output :type "MetaSoundOutput Structure (by ref)"))
  ;[1 1 1] Debug: volume output
)

(event `AnalyseSubmix`
  (params (Magnitude :type "Array of Float (single-precision) (by ref)"))
  (bind (_indexofmaxvalue _maxvalue) (`KismetMathLibrary.MaxOfFloatArray` Magnitude))
  ;[1 1 1] Getting highest magnitude frequency from array
  (set `self.CurrentNoteMagnitude` _maxvalue)
  ;[1 1 1] Calculating Current Note number
  (set `self.CurrentNoteNumber` (mod _indexofmaxvalue 12))
  (set `self.CurrentOctave` (/ _indexofmaxvalue 12))
  (set `self.CurrentMIDINote` (+ (`self.CurrentNoteNumber`) (* (+ (`self.CurrentOctave`) 2) 12)))
  ;[1 1 1] Getting current note name
  (set `self.CurentNoteName` (select `int` (`self.CurrentNoteNumber`) :`0` "C" :`1` "Db" :`2` "D" :`3` "Eb" :`4` "E" :`5` "F" :`6` "Gb" :`7` "G" :`8` "Ab" :`9` "A" :`10` "Bb" :`11` "B" :!type "EMusicalNoteName Enum"))
  ;[1 1 1] Getting colour associated with note number
  (set `self.CurrentColor` (`|GetArrayItem` (`self.Colors`) (`self.CurrentNoteNumber`)))
  (`self.UpdateNiagaraSystem`)
  ;[1 1 1] Checking if current note magnitude is higher than threshold
  (if (>= (`self.CurrentNoteMagnitude`) (`self.VolumeThreshold`))
    (`self.PitchDetectUpdate`)
    (else
      (`self.NoteEnd`))))

(event `UpdateNiagaraSystem`
  (`NiagaraComponent.SetVariableLinearColor` (`self.Niagara`) "NoteColor" (`self.CurrentColor`)))

(event `PitchDetectUpdate`
  ;[1 1 1] Broadcasting pitch detection update event - will be listened to by puzzles
  (`self.OnPitchDetectionUpdate` (`self.CurentNoteName`)))

(fn `UserConstructionScript`)